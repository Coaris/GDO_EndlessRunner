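; Actor component that pre-spawns a pool of reusable actors at its owner's location on BeginPlay.
; Each spawned actor gets its static mesh collision and shadow turned off, is attached to the owner, and receives a reference to the pool.
; The pool binds to each BP_ReusableActor's OnUsed event, which resets the actor to the owner's location and reattaches it for reuse.
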(event `self.ReceiveBeginPlay`
  (bind _returnvalue (`self.GetOwner`))
  ;[1 1 1] Spwan game objects and add them to themselves pool at the Game Instance initiation time
  (for _ (range (`self.AmountOfActors`))
    (bind _returnvalue_2 (`|SpawnActorFromClass` (`self.ReusableActorClass`) (`KismetMathLibrary.MakeTransform` (`Actor.K2_GetActorLocation` _returnvalue)) "Undefined" "MultiplyWithRoot" null null))
    (bind _returnvalue_3 (`Actor.GetComponentByClass` _returnvalue_2 "/Script/Engine.StaticMeshComponent"))
    ;[1 1 1] Set StaticMesh collision and shadow off
    (`PrimitiveComponent.SetCollisionEnabled` _returnvalue_3 "NoCollision")
    (`PrimitiveComponent.SetCastShadow` _returnvalue_3 false)
    ;[1 1 1] Attach to the pool in scene
    (`Actor.K2_AttachToActor` _returnvalue_2 _returnvalue "None" "KeepWorld" "KeepWorld" "KeepWorld" false)
    (bind _asbp_reusable_actor (cast `/Game/Coaris/BP/GameObjectPool/BP_ReusableActor` _returnvalue_2))
    ;[1 1 1] Give the reuasable actor this pool reference
    (set `/Game/Coaris/BP/GameObjectPool/BP_ReusableActor.Pool` self _asbp_reusable_actor)
    ;[1 1 1] Subscribe the OnUsed Event of reusable actors, and calling Reset Event of it
    (add `/Game/Coaris/BP/GameObjectPool/BP_ReusableActor.OnUsed` _asbp_reusable_actor (delegate `PutbackActor`))))

(event `PutbackActor`
  (params (ReusableActor :type "/Game/Coaris/BP/GameObjectPool/BP_ReusableActor Object Reference"))
  (bind _returnvalue (`self.GetOwner`))
  ;[1 1 1] Subscribe the OnUsed Event of reusable actors, and calling Reset Event of it
  ;;[1 1 1] Reset the actor
  (`/Game/Coaris/BP/GameObjectPool/BP_ReusableActor.ResetActor` ReusableActor (`Actor.K2_GetActorLocation` _returnvalue))
  ;;[1 1 1] Attach the pool in scene
  (`Actor.K2_AttachToActor` ReusableActor _returnvalue "None" "KeepWorld" "KeepWorld" "KeepWorld" false))
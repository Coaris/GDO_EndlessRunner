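; BP_RunnerTrack is a runner track actor that rotates around its roll axis when a lane change is requested, with comments naming the player as sender.
; OnChangeLane offsets the target angle 60 degrees by direction, then a timeline lerps the roll toward it.
; The current angle updates only when the timeline finishes.
; CalcTargetLane wraps an index across six lanes but is not called in this graph.
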(event `OnChangeLane`
  (params (IsRight :type Boolean))
  ;[1 1 1] Runner track will rotate, when get the rotation message form player.
  ;;[1 1 1] Calculate the lane target angle
  (`self.CalcTargetAngle` IsRight)
  ;;[1 1 1] Rotate the runner track
  (bind (_direction _lerpalpha) (`Timeline|LerpTimeline` :!via `PlayFromStart`)
    (:`Update`
      (`self.K2_SetActorRotation` (`KismetMathLibrary.MakeRotator` (`KismetMathLibrary.Lerp` (`self.CurrentAngle`) (`self.TargetAngle`) _lerpalpha))))
    (:`Finished`
      (set `self.CurrentAngle` (`self.TargetAngle`)))))

(fn `CalcTargetAngle`
  (params (IsRight :type Boolean))
  (if IsRight
    ;[1 1 1] Right
    (set `self.TargetAngle` (+ (`self.CurrentAngle`) 60.0))
    (else
      ;[1 1 1] left
      (set `self.TargetAngle` (- (`self.CurrentAngle`) 60.0)))))

(fn `CalcTargetLane`
  (params (IsRight :type Boolean))
  (returns (TargetLane :type Integer))
  (if IsRight
    ;[1 1 1] Change to right lane
    (bind _output_get (set `self.TargetLane` (mod (+ (`self.CurrentLane`) 1) 6)))
    (return _output_get)
    (else
      ;[1 1 1] Change to left lane
      (bind _output_get_2 (set `self.TargetLane` (mod (+ (`self.CurrentLane`) 5) 6)))
      (return _output_get_2))))

(fn `UserConstructionScript`)
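; BP_PoolComponent_Tile is a pool component that reuses tile actors to lay out a continuous chain of tiles.
; GetActorfromPool takes an actor from the reusable array into the using array, then places it at the stored target location with the given rotation and collision settings.
; Each BP_Tile's NextTilePosition becomes the next target location, and the placed actor leaves the reusable array.
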(event `self.ReceiveBeginPlay`
  (`parent.ReceiveBeginPlay`))

(event `self.GetActorFromPool`
  (params (AttachParent :type "Actor Object Reference") (TargetLocation :type "Vector Structure") (TargetRotation :type "Rotator Structure"))
  (bind _reusableactors (`self.ReusableActors`))
  ;[1 1 1] Get a reusable actor from reusable array and put it into using array
  (bind _reusableactor (`self.GetActorToUsingArray` AttachParent _reusableactors))
  ;;[1 1 1] Set actor's target location and so on
  (`/Game/Jiale_Chen/BP/ReusableActor/BP_ReusableActor.SetUsingActor` _reusableactor (`self.TargetLocation`) TargetRotation (`self.SMCollision`) (`self.ColCollision`))
  ;;[1 1 1] Set next location for next tile
  (bind _asbp_tile (cast `/Game/Jiale_Chen/BP/ReusableActor/BP_Tile` _reusableactor))
  (set `self.TargetLocation` (`SceneComponent.K2_GetComponentLocation` (`/Game/Jiale_Chen/BP/ReusableActor/BP_Tile.NextTilePosition` _asbp_tile)))
  ;;[1 1 1] Remove actor from reusable array
  (`KismetArrayLibrary.Array_RemoveItem` _reusableactors _reusableactor))
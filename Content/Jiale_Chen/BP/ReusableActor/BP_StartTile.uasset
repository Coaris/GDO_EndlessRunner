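; BP_StartTile is the opening tile of a runner track that seeds the track with pooled, reusable tiles.
; When the player overlaps StartCollision, it gets the BP_Tile pool from the game mode's PoolManager, sets the pool's target location to FirstTileLocation, and pulls StartTileCount tiles parented to the BP_RunnerTrack actor.
; Overlapping UsedCollision hides its mesh and disables its collisions rather than destroying it.
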(event `self.StartCollision.OnComponentBeginOverlap`
  (params (OverlappedComponent :type "PrimitiveComponent Object Reference") (OtherActor :type "Actor Object Reference") (OtherComp :type "PrimitiveComponent Object Reference") (OtherBodyIndex :type Integer) (bFromSweep :type Boolean) (SweepResult :type "HitResult Structure (by ref)"))
  ;[1 1 1] Set start reusable tiles from tile pool
  (cast `/Game/ThirdPerson/Blueprints/BP_ThirdPersonCharacter` OtherActor)
  (`|ExecutionSequence`
    (:`then_0`
      ;;[1 1 1] Get the Tile Pool reference
      (bind _asbp_third_person_game_mode (cast `/Game/ThirdPerson/Blueprints/BP_ThirdPersonGameMode` (`GameplayStatics.GetGameMode`)))
      (bind _pool (`/Game/Jiale_Chen/BP/ReusableActorPool/BP_PoolManager.Get Pool` (`/Game/ThirdPerson/Blueprints/BP_ThirdPersonGameMode.PoolManager` _asbp_third_person_game_mode) "/Game/Jiale_Chen/BP/ReusableActor/BP_Tile.BP_Tile_C"))
      (set `self.TilePool` _pool))
    (:`then_1`
      ;;[1 1 1] Get the Runner Track reference
      (bind _returnvalue (`GameplayStatics.GetActorOfClass` "/Game/Jiale_Chen/BP/BP_RunnerTrack.BP_RunnerTrack_C"))
      (set `self.RunnerTrack` _returnvalue))
    (:`then_2`
      ;;[1 1 1] Set initial reusable tile location
      (bind _asbp_pool_component_tile (cast `/Game/Jiale_Chen/BP/ReusableActorPool/BP_PoolComponent_Tile` (`self.TilePool`)))
      (set `/Game/Jiale_Chen/BP/ReusableActorPool/BP_PoolComponent_Tile.TargetLocation` (`SceneComponent.K2_GetComponentLocation` (`self.FirstTileLocation`)) _asbp_pool_component_tile))
    (:`then_3`
      ;;[1 1 1] Set some tiles from tile pool
      (for _ (range 1 (+ (`self.StartTileCount`) 1))
        (`/Game/Jiale_Chen/BP/ReusableActorPool/BP_PoolComponent.GetActorFromPool` :`self` (`self.TilePool`) :`AttachParent` (`self.RunnerTrack`))))))

(event `self.UsedCollision.OnComponentBeginOverlap`
  (params (OverlappedComponent :type "PrimitiveComponent Object Reference") (OtherActor :type "Actor Object Reference") (OtherComp :type "PrimitiveComponent Object Reference") (OtherBodyIndex :type Integer) (bFromSweep :type Boolean) (SweepResult :type "HitResult Structure (by ref)"))
  (bind _staticmesh (`self.StaticMesh`))
  ;[1 1 1] Hidden in game when player pass this tile
  (cast `/Game/ThirdPerson/Blueprints/BP_ThirdPersonCharacter` OtherActor)
  (`PrimitiveComponent.SetCollisionEnabled` _staticmesh "NoCollision")
  (`SceneComponent.SetHiddenInGame` _staticmesh true false)
  (`PrimitiveComponent.SetCollisionEnabled` (`self.StartCollision`) "NoCollision")
  (`PrimitiveComponent.SetCollisionEnabled` (`self.UsedCollision`) "NoCollision"))

(fn `UserConstructionScript`)
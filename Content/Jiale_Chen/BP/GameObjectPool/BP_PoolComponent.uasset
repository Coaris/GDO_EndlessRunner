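; Object pool component that registers with its owning BP_PoolManager and recycles BP_ReusableActor instances.
; On BeginPlay it pre-spawns a set number of actors at the owner, attaches them and binds their OnUsed event to return them to the pool.
; Requests take an available actor, optionally shuffled, place and reparent it, and track it as in use.
; Returned actors are reset and reattached; an empty pool does not grow.
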(event `self.ReceiveBeginPlay`
  (bind _returnvalue (`self.GetOwner`))
  ;[1 1 1] Add self to GameObjectPool(Manager)'s Pool Array
  (bind _asbp_pool_manager (cast `/Game/Jiale_Chen/BP/GameObjectPool/BP_PoolManager` (`self.GetOwner`)))
  (`KismetArrayLibrary.Array_Add` (`/Game/Jiale_Chen/BP/GameObjectPool/BP_PoolManager.PoolArray` _asbp_pool_manager) self)
  ;[1 1 1] Spwan game objects and add them to themselves pool at the Game Instance initiation time
  (for _ (range (`self.AmountOfActors`))
    (bind _returnvalue_2 (`|SpawnActorFromClass` (`self.ReusableActorClass`) (`KismetMathLibrary.MakeTransform` (`Actor.K2_GetActorLocation` _returnvalue)) "Undefined" "MultiplyWithRoot" null null))
    ;[1 1 1] Attach to the pool in scene
    (`Actor.K2_AttachToActor` _returnvalue_2 _returnvalue "None" "KeepWorld" "KeepWorld" "KeepWorld" false)
    ;[1 1 1] Initialize Actor
    (bind _asbp_reusable_actor (cast `/Game/Jiale_Chen/BP/GameObjectPool/BP_ReusableActor` _returnvalue_2))
    (`/Game/Jiale_Chen/BP/GameObjectPool/BP_ReusableActor.InitializeActor` _asbp_reusable_actor self)
    ;[1 1 1] Subscribe the OnUsed Event of reusable actors, and calling Reset Event of it
    (add `/Game/Jiale_Chen/BP/GameObjectPool/BP_ReusableActor.OnUsed` _asbp_reusable_actor (delegate `PutbackActorToPool`))
    ;;[1 1 1] Add actor to array
    (`KismetArrayLibrary.Array_Add` (`self.ReusableActors`) _asbp_reusable_actor)))

(event `PutbackActorToPool`
  (params (ReusableActor :type "/Game/Jiale_Chen/BP/GameObjectPool/BP_ReusableActor Object Reference"))
  (bind _returnvalue (`self.GetOwner`))
  ;[1 1 1] Subscribe the OnUsed Event of reusable actors, and calling Reset Event of it
  ;;[1 1 1] Reset the actor
  (`/Game/Jiale_Chen/BP/GameObjectPool/BP_ReusableActor.ResetActor` ReusableActor (`Actor.K2_GetActorLocation` _returnvalue))
  ;;[1 1 1] Attach the pool in scene
  (`Actor.K2_AttachToActor` ReusableActor _returnvalue "None" "KeepWorld" "KeepWorld" "KeepWorld" false)
  ;;[1 1 1] Change array from inusing array to resuable array
  (`KismetArrayLibrary.Array_Add` (`self.ReusableActors`) ReusableActor)
  (`KismetArrayLibrary.Array_RemoveItem` (`self.UsingActors`) ReusableActor))

(event `GetActorFromPool`
  (params (AttachParent :type "Actor Object Reference"))
  (bind _reusableactors (`self.ReusableActors`))
  ;[1 1 1] Get reusable actor form reusable array and put it into using array
  (bind _reusableactor (`self.PutActorToUsingArray` AttachParent _reusableactors))
  ;;[1 1 1] Remove actor from reusable array
  (`KismetArrayLibrary.Array_RemoveItem` _reusableactors _reusableactor))

(fn `PutActorToUsingArray`
  (params (AttachParent :type "Actor Object Reference") (ReusableActorsArray :type "Array of /Game/Jiale_Chen/BP/GameObjectPool/BP_ReusableActor Object Reference"))
  (returns (ReusableActor :type "/Game/Jiale_Chen/BP/GameObjectPool/BP_ReusableActor Object Reference"))
  (bind _output (`|GetArrayItem` ReusableActorsArray))
  ;[1 1 1] Check is not empty
  (if (`KismetArrayLibrary.Array_IsNotEmpty` ReusableActorsArray)
    ;[1 1 1] Check if it need shuffle
    (if (`self.IsNeedShuffle`)
      (`KismetArrayLibrary.Array_Shuffle` ReusableActorsArray))
    ;[1 1 1] Change array from reusable array to inusing array
    (`KismetArrayLibrary.Array_Add` (`self.UsingActors`) _output)
    ;[1 1 1] Set actor's target location and so on
    (`/Game/Jiale_Chen/BP/GameObjectPool/BP_ReusableActor.SetUsingActor` _output (`self.TargetLoaction`) (`self.TargetRotation`) (`self.SMCollision`) (`self.ColCollision`))
    (`Actor.K2_AttachToActor` _output AttachParent "None" "KeepWorld" "KeepWorld" "KeepWorld" true)
    (return _output)))
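; Reusable actor for an object pool, with a static mesh and a collision component.
; InitializeActor hides the mesh, disables shadows and collision, and stores the pool reference.
; SetUsingActor places the actor at a given transform, shows the mesh and applies the requested collision modes.
; ResetActor, called when the pool takes it back, moves it to a given location, zeroes rotation, and hides and disables it again.
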(event `ResetActor`
  (params (TargetLocation :type "Vector Structure"))
  (bind _staticmesh (`self.StaticMesh`))
  ;[1 1 1] Reset the actor when it be put back to the pool. Being called when pool put this actor back.
  (`|ExecutionSequence`
    (:`then_0`
      ;;[1 1 1] Transform
      (`self.K2_SetActorLocation` TargetLocation)
      (`self.K2_SetActorRotation` (struct)))
    (:`then_1`
      ;;[1 1 1] Static Mesh
      (`PrimitiveComponent.SetCollisionEnabled` _staticmesh "NoCollision")
      (`SceneComponent.SetHiddenInGame` _staticmesh true true))
    (:`then_2`
      ;;[1 1 1] Collision
      (`PrimitiveComponent.SetCollisionEnabled` (`self.Collision`) "NoCollision"))))

(event `InitializeActor`
  (params (Pool :type "/Game/Jiale_Chen/BP/GameObjectPool/BP_PoolComponent Object Reference"))
  (bind _staticmesh (`self.StaticMesh`))
  ;[1 1 1] Initalize
  (`|ExecutionSequence`
    (:`then_0`
      ;;[1 1 1] Initialize Static Mesh
      (`PrimitiveComponent.SetCollisionEnabled` _staticmesh "NoCollision")
      (`PrimitiveComponent.SetCastShadow` _staticmesh false)
      (`SceneComponent.SetHiddenInGame` _staticmesh true true))
    (:`then_1`
      ;;[1 1 1] Collision
      (`PrimitiveComponent.SetCollisionEnabled` (`self.Collision`) "NoCollision"))
    (:`then_2`
      ;;[1 1 1] Get Pool reference
      (set `self.Pool` Pool))))

(event `SetUsingActor`
  (params (TargetLocation :type "Vector Structure") (TargetRotation :type "Rotator Structure") (SM_CollisionEnabled :type "ECollisionEnabled Enum" :default "NoCollision") (Collision_CollisionEnabled :type "ECollisionEnabled Enum" :default "NoCollision"))
  (bind _staticmesh (`self.StaticMesh`))
  ;[1 1 1] Set the actor Location and Rotation when it be gotten from the pool.
  (`|ExecutionSequence`
    (:`then_0`
      ;;[1 1 1] Transform
      (`self.K2_SetActorLocation` TargetLocation)
      (`self.K2_SetActorRotation` TargetRotation))
    (:`then_1`
      ;;[1 1 1] Static Mesh
      (`PrimitiveComponent.SetCollisionEnabled` _staticmesh SM_CollisionEnabled)
      (`SceneComponent.SetHiddenInGame` _staticmesh false true))
    (:`then_2`
      ;;[1 1 1] Collision
      (`PrimitiveComponent.SetCollisionEnabled` (`self.Collision`) Collision_CollisionEnabled))))

(fn `UserConstructionScript`)